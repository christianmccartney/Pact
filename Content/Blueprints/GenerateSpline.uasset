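; GenerateSpline Blueprint that shapes a flat, quarter-turn spiral path from a start location, radius, variance, length and spin direction.
; GenerateSpline picks one of its preset splines by length, repositions each point and returns that spline.
; CoolMath and CoolMath2 supply direction-dependent corner offsets and axis-aligned tangents, while each radius change shrinks to a third of the previous one.
; The construction script and events are empty, leaving generation to callers.
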(fn `CoolMath`
  (params (Select :type Integer) (I :type Integer))
  (returns (X :type Integer) (Y :type Integer))
  (locals (MX :type Integer :default 0) (MY :type Integer :default 0))
  (bind _returnvalue (mod I 4))
  (switch `int` (`KismetMathLibrary.SignOfInteger` Select)
    (:`-1`
      (switch `int` _returnvalue
        (:`0`
          (set `local.MX` 1 :!label _label)
          (set `local.MY` 1))
        (:`1`
          (set `local.MX` 1)
          (set `local.MY` -1))
        (:`2`
          (set `local.MX` -1)
          (set `local.MY` -1))
        (:`3`
          (set `local.MX` -1)
          (set `local.MY` 1))
        (:`4`
          (goto _label))))
    (:`0`
      (switch `int` _returnvalue
        (:`1`
          (set `local.MX` 1)
          (set `local.MY` 0))
        (:`2`
          (set `local.MX` 0)
          (set `local.MY` 1))
        (:`3`
          (set `local.MX` -1)
          (set `local.MY` -1))
        (:`4`
          (set `local.MX` 0)
          (set `local.MY` -1))))
    (:`1`
      (switch `int` _returnvalue
        (:`0`
          (set `local.MX` 1 :!label _label_2)
          (set `local.MY` -1))
        (:`1`
          (set `local.MX` 1)
          (set `local.MY` 1))
        (:`2`
          (set `local.MX` -1)
          (set `local.MY` 1))
        (:`3`
          (set `local.MX` -1)
          (set `local.MY` -1))
        (:`4`
          (goto _label_2)))))
  (return (`local.MX`) (`local.MY`)))

(fn `CoolMath2`
  (params (Select :type Integer) (I :type Integer))
  (returns (X :type Integer) (Y :type Integer))
  (locals (MX :type Integer :default 0) (MY :type Integer :default 0))
  (bind _returnvalue (mod I 4))
  (switch `int` (`KismetMathLibrary.SignOfInteger` Select)
    (:`-1`
      (switch `int` _returnvalue
        (:`0`
          (set `local.MX` 0)
          (set `local.MY` 1))
        (:`1`
          (set `local.MX` 1)
          (set `local.MY` 0))
        (:`2`
          (set `local.MX` 0)
          (set `local.MY` -1))
        (:`3`
          (set `local.MX` -1)
          (set `local.MY` 0)))
      (return (`local.MX`) (`local.MY`)))
    (:`0`
      (switch `int` _returnvalue))
    (:`1`
      (switch `int` _returnvalue
        (:`0`
          (set `local.MX` 0)
          (set `local.MY` -1))
        (:`1`
          (set `local.MX` 1)
          (set `local.MY` 0))
        (:`2`
          (set `local.MX` 0)
          (set `local.MY` 1))
        (:`3`
          (set `local.MX` -1)
          (set `local.MY` 0)))
      (return (`local.MX`) (`local.MY`)))))

(fn `GenerateSpline`
  (params (Location :type "Vector Structure") (Variance :type "Float (double-precision)") (Radius :type "Float (double-precision)") (Length :type Integer) (`Spin Direction` :type Integer))
  (returns (NewParam :type "SplineComponent Object Reference"))
  (locals (RefSpline :type "SplineComponent Object Reference"))
  (bind _spin_direction (`local.Spin Direction`))
  (bind _old_radius (`self.Old Radius`))
  (bind _returnvalue (+ (`self.Point Index`) 1))
  (switch `int` Length
    (:`2`
      (set `local.RefSpline` (`self.Spline2`)))
    (:`3`
      (set `local.RefSpline` (`self.Spline3`)))
    (:`4`
      (set `local.RefSpline` (`self.Spline4`)))
    (:`5`
      (set `local.RefSpline` (`self.Spline5`)))
    (:`6`
      (set `local.RefSpline` (`self.Spline6`))))
  (set `self.Radius Variance` (* -1 Variance))
  (set `self.Old Radius` Radius)
  (set `self.Old X` (.x Location))
  (set `self.Old Y` (.y Location))
  (for _index (range (+ (`local.Length`) 1))
    (set `self.Point Index` _index)
    (`SplineComponent.SetLocationAtSplinePoint` (`local.RefSpline`) (`self.Point Index`) (`KismetMathLibrary.MakeVector` (`self.Old X`) (`self.Old Y`)) "World" true)
    (bind (_x _y) (`self.CoolMath` _spin_direction _returnvalue))
    (bind (_x_2 _y_2) (`self.CoolMath2` _spin_direction _returnvalue))
    (set `self.New X` (+ (* _x _old_radius) (`self.Old X`)))
    (set `self.New Y` (+ (* _y _old_radius) (`self.Old Y`)))
    (`SplineComponent.SetTangentsAtSplinePoint` (`local.RefSpline`) (`self.Point Index`) (`KismetMathLibrary.MakeVector` (* (* _x_2 1.5) (`self.Old Radius`)) (* (* _y_2 1.5) (`self.Old Radius`))) (`KismetMathLibrary.MakeVector` (* (* _x_2 1.5) (`self.Old Radius`)) (* (* _y_2 1.5) (`self.Old Radius`))) "Local" true)
    (set `self.Old Radius` (- (`self.Old Radius`) (`self.Radius Variance`)))
    (set `self.Radius Variance` (/ (`self.Radius Variance`) 3.0))
    (set `self.Old X` (`self.New X`))
    (set `self.Old Y` (`self.New Y`)))
  (return (`local.RefSpline`)))

(fn `UserConstructionScript`)